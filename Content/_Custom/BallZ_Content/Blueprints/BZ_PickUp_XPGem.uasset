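; BallZ XP gem pickup that the player collects on touch.
; On BeginPlay it rolls a random XP value within its min/max range and scales itself by that value's clamped ratio to the maximum.
; Two chained MoveComponentTo events alternate endlessly to create an eased vertical bob.
; When the player pawn overlaps it, the gem passes itself to the pawn through InteractionMessage, then destroys itself.
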(event Custom|Move%20Up
  ;[0.15 0.15 0.15 0.5] Move the Sphere Component to create a "bobbing" effect
  (Components|MoveComponentTo 0 "0.000000,0.000000,-25.000000" "0, 0, 0" true true 0.33 false)
  (CallFunction|MoveDown))

(event Custom|Move%20Down
  ;[0.15 0.15 0.15 0.5] Move the Sphere Component to create a "bobbing" effect
  (Components|MoveComponentTo 0 "0.000000,0.000000,25.000000" "0, 0, 0" true true 0.33 false)
  (CallFunction|MoveUp))

(event Collision|EventActorBeginOverlap
  (params (OtherActor :type Actor%20Object%20Reference))
  ;[0.15 0.15 0.15 0.5] If Player overlaps Collision, enable Pickup logic
  (if (== OtherActor (Game|Player|GetPlayerPawn 0))
    (Class|BPIBZ|Interaction(Message) (Game|Player|GetPlayerPawn 0) self)
    (Actor|DestroyActor)))

(event EventBeginPlay
  ;[0.15 0.15 0.15 0.5] Move the Sphere Component to create a "bobbing" effect
  (bind _xpvalue (CallFunction|RandomXpValue))
  (Transformation|SetWorldScale3D (Variables|Default|GetScene) (Math|Conversions|ToVector(Float) (Math|Float|Clamp(Float) (/ _xpvalue (Variables|Default|GetXpMax)) 0.25 1.0)))
  (CallFunction|MoveUp))

(fn ConstructionScript)

(fn RandomXpValue
  (bind _output_get (Variables|Default|SetXpValue (Math|Random|RandomFloatinRange (Variables|Default|GetXpMin) (Variables|Default|GetXpMax))))
  (return _output_get))