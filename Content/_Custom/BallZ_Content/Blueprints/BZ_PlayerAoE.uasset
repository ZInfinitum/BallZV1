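; BZ_PlayerAoE is a self-destroying player area-of-effect attack that hits BP_TwinStickNPC enemies inside its collision sphere.
; A looping timer repeatedly sends ProjectileImpactMessage to overlapping NPCs while AOEActive is set, catching stragglers.
; A one-shot timer starts a Timeline driving global time dilation and, after a short delay, removes the visual sphere and stops damage.
; When the Timeline finishes, it restores normal time and destroys the actor.
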(event Custom|AOE%20Attack
  ;[0.15 0.15 0.15 0.5] Get All Actors inside Sphere Collision and Damage Them. We loop this to catch any stragglers.
  (if (Variables|AOE|GetAOE%20Active)
    (for _array_element (Collision|GetOverlappingActors (Variables|Default|GetSphere) "/Game/_Custom/BallZ_Content/Blueprints/AI/BP_TwinStickNPC.BP_TwinStickNPC_C" :!class /Script/Engine.PrimitiveComponent)
      (Class|BPIBZ|ProjectileImpact(Message) _array_element "0, 0, 0"))))

(event Custom|AOE%20Structure
  (Utilities|FlowControl|Sequence
    (:then_0
      ;[0.15 0.15 0.15 0.5] Remove AOE visuals and stop checking for enemies
      (Utilities|FlowControl|Delay 0.5)
      (Components|DestroyComponent (Variables|Default|GetSphere_Visual))
      (Variables|AOE|SetAOE%20Active false))
    (:then_1
      ;[0.15 0.15 0.15 0.5] Manage Time Dilation via a Timeline during AOE attack, cleanup after
      (bind _timedilation (Timeline|Timeline Play)
        (:Update
          (Utilities|Time|SetGlobalTimeDilation _timedilation))
        (:Finished
          (Utilities|Time|SetGlobalTimeDilation 1.0)
          (Actor|DestroyActor))))))

(event EventBeginPlay
  ;[0.15 0.15 0.15 0.502] Pre-Attack Delay
  (Utilities|Time|SetTimerbyEvent (delegate Custom|AOE%20Attack) 0.33 true)
  (Utilities|Time|SetTimerbyEvent (delegate Custom|AOE%20Structure) 0.5))

(fn ConstructionScript)