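; Base pickup actor for BallZ that bobs in place until the player touches it.
; MoveUp and MoveDown call each other through eased MoveComponentTo moves, looping the Sphere's vertical bob from BeginPlay.
; When player 0's pawn overlaps it, the pickup sends that pawn an InteractionMessage with itself as the argument, then destroys itself, leaving the pickup's effect to the receiver.
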(event Custom|Move%20Up
  ;[0.15 0.15 0.15 0.5] Move the Sphere Component to create a "bobbing" effect
  (Components|MoveComponentTo (Variables|Default|GetSphere) "0.000000,0.000000,-25.000000" "0, 0, 0" true true 0.33 false)
  (CallFunction|MoveDown))

(event Custom|Move%20Down
  ;[0.15 0.15 0.15 0.5] Move the Sphere Component to create a "bobbing" effect
  (Components|MoveComponentTo (Variables|Default|GetSphere) "0.000000,0.000000,25.000000" "0, 0, 0" true true 0.33 false)
  (CallFunction|MoveUp))

(event Collision|EventActorBeginOverlap
  (params (OtherActor :type Actor%20Object%20Reference))
  ;[0.15 0.15 0.15 0.5] If Player overlaps Collision, enable Pickup logic
  (if (== OtherActor (Game|Player|GetPlayerPawn 0))
    (Class|BPIBZ|Interaction(Message) (Game|Player|GetPlayerPawn 0) self)
    (Actor|DestroyActor)))

(event EventBeginPlay
  ;[0.15 0.15 0.15 0.5] Move the Sphere Component to create a "bobbing" effect
  (CallFunction|MoveUp))

(fn ConstructionScript)